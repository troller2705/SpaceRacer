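; BP_LapTrigger is the lap line trigger for a vehicle game, handling lap timing, lap counting and the best-time record.
; The first overlap by any actor starts timing, and Tick accumulates LapTime on VehicleAdvGameMode.
; Later overlaps save faster times to the "BestTime" slot, reloaded on BeginPlay, and reset the timer.
; Every overlap increments LapCounter, opening the Gameover level once it exceeds TotalLaps.
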(event `self.ReceiveBeginPlay`
  (bind _asvehicle_adv_game_mode (cast `/Game/VehicleTemplate/Blueprints/VehicleAdvGameMode` (`GameplayStatics.GetGameMode`)))
  (bind _output_get (set `self.GameMode` _asvehicle_adv_game_mode))
  (bind _returnvalue (`GameplayStatics.DoesSaveGameExist` "BestTime"))
  (if _returnvalue
    (bind _returnvalue_2 (`GameplayStatics.LoadGameFromSlot` "BestTime"))
    (bind _asbp_save_game (cast `/Game/Blueprints/BP_SaveGame` _returnvalue_2))
    (set `/Game/VehicleTemplate/Blueprints/VehicleAdvGameMode.BestLapTime` (`/Game/Blueprints/BP_SaveGame.BestTime` _asbp_save_game) _output_get)))

(event `self.ReceiveActorBeginOverlap`
  (params (OtherActor :type "Actor Object Reference"))
  (bind _gamemode (`self.GameMode`))
  (bind _lapcounter (`/Game/VehicleTemplate/Blueprints/VehicleAdvGameMode.LapCounter` _gamemode))
  (bind _laptime (`/Game/VehicleTemplate/Blueprints/VehicleAdvGameMode.LapTime` _gamemode))
  (if (`self.IsTiming`)
    (`/Engine/EditorBlueprintResources/StandardMacros.CompareFloat` _laptime (`/Game/VehicleTemplate/Blueprints/VehicleAdvGameMode.BestLapTime` _gamemode)
      (:`>`
        _)
      (:`==`
        _)
      (:`<`
        (bind _output_get (set `/Game/VehicleTemplate/Blueprints/VehicleAdvGameMode.BestLapTime` _laptime _gamemode))
        (bind _returnvalue (`GameplayStatics.CreateSaveGameObject` "/Game/Blueprints/BP_SaveGame.BP_SaveGame_C"))
        (set `/Game/Blueprints/BP_SaveGame.BestTime` _output_get _returnvalue)
        (`GameplayStatics.SaveGameToSlot` _returnvalue "BestTime")))
    (set `/Game/VehicleTemplate/Blueprints/VehicleAdvGameMode.LapTime` 0.0 _gamemode)
    (else
      (set `self.IsTiming` true)
      (set `/Game/VehicleTemplate/Blueprints/VehicleAdvGameMode.LapTime` 0.0 _gamemode)))
  (bind _result (`/Engine/EditorBlueprintResources/StandardMacros.IncrementInt` _lapcounter)
    (:`  `
      (set `/Game/VehicleTemplate/Blueprints/VehicleAdvGameMode.LapCounter` _result _gamemode)
      (if (> _lapcounter (`/Game/VehicleTemplate/Blueprints/VehicleAdvGameMode.TotalLaps` _gamemode))
        (`GameplayStatics.OpenLevelBySoftObjectPtr` "/Game/Map/Gameover.Gameover")))))

(event `self.ReceiveTick`
  (params (DeltaSeconds :type "Float (single-precision)"))
  (bind _gamemode (`self.GameMode`))
  (if (`self.IsTiming`)
    (set `/Game/VehicleTemplate/Blueprints/VehicleAdvGameMode.LapTime` (+ (`GameplayStatics.GetWorldDeltaSeconds`) (`/Game/VehicleTemplate/Blueprints/VehicleAdvGameMode.LapTime` _gamemode)) _gamemode)))

(fn `UserConstructionScript`)