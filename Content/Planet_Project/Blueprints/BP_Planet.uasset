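; Configurable planet actor that orbits an optional center actor and can carry its own nebula and star skybox dome.
; The construction script feeds exposed settings into dynamic materials for surface, clouds and atmosphere, sky atmosphere and volumetric cloud components, and a shared cloud parameter collection.
; It also sets global render console variables for volumetric cloud quality.
; Tick re-orthogonalizes the orbit axis, follows the moving center, and spins the high-geometry mesh when used.
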(event `OrthogonalizeAxis`
  (bind _returnvalue (- (`self.K2_GetActorLocation`) (`self.CenterLocation`)))
  (set `self.Orbit_Axis` (`KismetMathLibrary.Normal` (`KismetMathLibrary.Cross_VectorVector` _returnvalue (`KismetMathLibrary.Cross_VectorVector` (`self.Orbit_Axis`) _returnvalue)))))

(event `self.ReceiveBeginPlay`
  (`|ExecutionSequence`
    (:`then_0`
      (bind _center_of_orbit (`self.Center_of_Orbit`)
        (:`then`
          (set `self.CenterLocation` (`self.K2_GetActorLocation` _center_of_orbit)))
        (:`else`)))
    (:`then_1`
      (set `self.OldCenterLocation` (`self.CenterLocation`)))))

(event `self.ReceiveTick`
  (params (DeltaSeconds :type "Float (single-precision)"))
  (`|ExecutionSequence`
    (:`then_0`
      (bind _center_of_orbit (`self.Center_of_Orbit`)
        (:`then`
          (set `self.CenterLocation` (`self.K2_GetActorLocation` _center_of_orbit)))
        (:`else`)))
    (:`then_1`
      (`self.OrthogonalizeAxis`)
      (`self.K2_SetActorLocation` (+ (`KismetMathLibrary.RotateAngleAxis` (- (`self.K2_GetActorLocation`) (`self.OldCenterLocation`)) (* DeltaSeconds (`self.Orbit_Speed`)) (`self.Orbit_Axis`)) (`self.CenterLocation`)))
      (set `self.OldCenterLocation` (`self.CenterLocation`))
      ;[1 1 1] Rotate_High_Geo_Planet
      (if (`self.High_Geometry_Planet?`)
        (`SceneComponent.K2_AddLocalRotation` (`self.SM_Planet_Geometry_Detail`) (`KismetMathLibrary.MakeRotator` 0.0 0.0 (* (`GameplayStatics.GetWorldDeltaSeconds`) (`self.Planet_High_Geometry_Rotation_Speed`))) false false)))))

(fn `UserConstructionScript`
  (bind _sm_skybox_dome (`self.SM_Skybox_Dome`))
  (bind _volumetriccloud (`self.VolumetricCloud`))
  (bind _sm_planet_clouds (`self.SM_Planet_Clouds`))
  (bind _sm_planet_atmosphere (`self.SM_Planet_Atmosphere`))
  (bind _skyatmosphere (`self.SkyAtmosphere`))
  (bind _mid_cloud (`self.MID_Cloud`))
  (bind _mid_cloud_shadows (`self.MID_Cloud_Shadows`))
  (bind _mid_planet (`self.MID_Planet`))
  (bind _mid_planet_atmosphere (`self.MID_Planet_Atmosphere`))
  (`|ExecutionSequence`
    (:`then_0`
      (if (`self.High_Geometry_Planet?`)
        (`StaticMeshComponent.SetStaticMesh` (`self.SM_Planet_Geometry_Detail`) (`self.High_Geo_Mesh`))
        (`SceneComponent.SetVisibility` (`self.SM_Planet_Sphere`) false false)
        (`SceneComponent.SetVisibility` (`self.SM_Planet_Geometry_Detail`) true false)
        (bind _returnvalue (`PrimitiveComponent.CreateDynamicMaterialInstance` (`self.SM_Planet_Geometry_Detail`) 0 (`self.Planet_Material`) "None"))
        (set `self.MID_Planet` _returnvalue)
        ;[1 1 1] Explain here
        (set `self.Planet_Rotation_Speed` 0.0)
        (else
          (`SceneComponent.SetVisibility` (`self.SM_Planet_Sphere`) true false)
          (`SceneComponent.SetVisibility` (`self.SM_Planet_Geometry_Detail`) false false)
          (bind _returnvalue_2 (`PrimitiveComponent.CreateDynamicMaterialInstance` (`self.SM_Planet_Sphere`) 0 (`self.Planet_Material`) "None"))
          (set `self.MID_Planet` _returnvalue_2)))
      (bind _returnvalue_3 (`PrimitiveComponent.CreateDynamicMaterialInstance` (`self.SM_Planet_Clouds`) 0 (`self.Cloud_Material`) "None"))
      (set `self.MID_Cloud` _returnvalue_3)
      (bind _returnvalue_4 (`PrimitiveComponent.CreateDynamicMaterialInstance` (`self.SM_Planet_Cloud_Shadows`) 0 (`self.Cloud_Shadow_Material`) "None"))
      (set `self.MID_Cloud_Shadows` _returnvalue_4)
      (bind _returnvalue_5 (`PrimitiveComponent.CreateDynamicMaterialInstance` (`self.SM_Planet_Atmosphere`) 0 (`self.Planet_Atmosphere`) "None"))
      (set `self.MID_Planet_Atmosphere` _returnvalue_5))
    (:`then_1`
      ;[1 1 1] Material_Controls_Planet_Clouds
      (`MaterialInstanceDynamic.SetScalarParameterValue` _mid_planet "Normal_Intensity" (`self.Planet_Normal_Intensity`))
      (`MaterialInstanceDynamic.SetScalarParameterValue` _mid_planet "Planet_Rotation_Speed" (`self.Planet_Rotation_Speed`))
      (`MaterialInstanceDynamic.SetScalarParameterValue` _mid_planet "Planet_Color_Blend_Intensity" (`self.Planet_Color_Blend_Intensity`))
      (`MaterialInstanceDynamic.SetVectorParameterValue` _mid_planet "Planet_Color_Blend" (`KismetMathLibrary.Conv_ColorToLinearColor` (`self.Planet_Color_Blend`)))
      (`MaterialInstanceDynamic.SetTextureParameterValue` _mid_planet "Diffuse Texture" (`self.Planet_Texture`))
      (`MaterialInstanceDynamic.SetTextureParameterValue` _mid_planet "Normal_Texture" (`self.Planet_Normal`))
      (if (`self.City_Lights?`)
        (`MaterialInstanceDynamic.SetScalarParameterValue` _mid_planet "City_Lights" (`self.City_Lights_On`))
        (else
          (`MaterialInstanceDynamic.SetScalarParameterValue` _mid_planet "City_Lights" (`self.City_Lights_Off`))))
      (`MaterialInstanceDynamic.SetTextureParameterValue` _mid_planet "Emissive_Texture" (`self.Planet_City_Lights`))
      (if (`self.Roughness_Texture?`)
        (`MaterialInstanceDynamic.SetScalarParameterValue` _mid_planet "Roughness_Switch" (`self.Roughness_On`))
        (else
          (`MaterialInstanceDynamic.SetScalarParameterValue` _mid_planet "Roughness_Switch" (`self.Roughness_Off`))))
      (`MaterialInstanceDynamic.SetScalarParameterValue` _mid_planet "Roughness_Weight" (`self.Roughness_Weight`))
      (`MaterialInstanceDynamic.SetTextureParameterValue` _mid_planet "Roughness Texture" (`self.Planet_Roughness`))
      (`MaterialInstanceDynamic.SetTextureParameterValue` _mid_planet "Specular Texture" (`self.Planet_Specular`))
      (if (`self.Specular_Texture?`)
        (`MaterialInstanceDynamic.SetScalarParameterValue` _mid_planet "Specular_Switch" (`self.Specular_On`))
        (else
          (`MaterialInstanceDynamic.SetScalarParameterValue` _mid_planet "Specular_Switch" (`self.Specular_Off`))))
      (`MaterialInstanceDynamic.SetScalarParameterValue` _mid_planet "Specular Weight" (`self.Specular_Weight`)))
    (:`then_2`
      (if (`self.Simple_Clouds?`)
        (`SceneComponent.SetVisibility` _sm_planet_clouds true false)
        (`SceneComponent.SetVisibility` (`self.SM_Planet_Cloud_Shadows`) true false)
        (else
          (`SceneComponent.SetVisibility` _sm_planet_clouds false false)
          (`SceneComponent.SetVisibility` (`self.SM_Planet_Cloud_Shadows`) false false)))
      (`|ExecutionSequence`
        (:`then_0`
          (`MaterialInstanceDynamic.SetScalarParameterValue` _mid_cloud "Cloud_Rotation_Speed" (`self.Cloud_Rotation_Speed`))
          (`MaterialInstanceDynamic.SetScalarParameterValue` _mid_cloud "Normal_Intensity" (`self.Cloud_Normal_Intensity`))
          (`MaterialInstanceDynamic.SetVectorParameterValue` _mid_cloud "Cloud Color" (`KismetMathLibrary.Conv_ColorToLinearColor` (`self.Cloud_Color`)))
          (`MaterialInstanceDynamic.SetScalarParameterValue` _mid_cloud "Cloud_Opacity" (`self.Cloud_Opacity`)))
        (:`then_1`
          (`MaterialInstanceDynamic.SetScalarParameterValue` _mid_cloud_shadows "Cloud_Shadows_Rotation_Speed" (`self.Cloud_Rotation_Speed`))
          (`MaterialInstanceDynamic.SetVectorParameterValue` _mid_cloud_shadows "Cloud_Shadow_Color" (`KismetMathLibrary.Conv_ColorToLinearColor` (`self.Cloud_Shadow_Color`)))
          (`MaterialInstanceDynamic.SetScalarParameterValue` _mid_cloud_shadows "Shadow_Opacity" (`KismetMathLibrary.FClamp` (`self.Coud_Shadow_Opacity`) -2.0)))))
    (:`then_3`
      (if (`self.Simple_Atmosphere?`)
        (`SceneComponent.SetVisibility` _sm_planet_atmosphere true false)
        (else
          (`SceneComponent.SetVisibility` _sm_planet_atmosphere false false)))
      (`MaterialInstanceDynamic.SetScalarParameterValue` _mid_planet_atmosphere "Atmosphere_Night_Time" (`self.Atmosphere_Night_Time`))
      (`MaterialInstanceDynamic.SetScalarParameterValue` _mid_planet_atmosphere "Atmosphere Edge Clamp" (`self.Atmosphere Edge Clamp`))
      (`MaterialInstanceDynamic.SetScalarParameterValue` _mid_planet_atmosphere "Atmosphere Falloff" (`self.Atmosphere Falloff`))
      (`MaterialInstanceDynamic.SetScalarParameterValue` _mid_planet_atmosphere "Atmosphere Intesity" (`self.Atmosphere Intesity`))
      (`MaterialInstanceDynamic.SetVectorParameterValue` _mid_planet_atmosphere "Atmosphere Color" (`KismetMathLibrary.Conv_ColorToLinearColor` (`self.Atmosphere_Color`))))
    (:`then_4`
      (if (`self.Volumetric_Atmosphere?`)
        (`SceneComponent.SetVisibility` _skyatmosphere true false)
        (else
          (`SceneComponent.SetVisibility` _skyatmosphere false false)))
      (`SkyAtmosphereComponent.SetAtmosphereHeight` _skyatmosphere (`self.Atmosphere_Hieght`))
      (`SkyAtmosphereComponent.SetBottomRadius` _skyatmosphere (`self.Atmosphere_Ground_Radius`))
      (`SkyAtmosphereComponent.SetRayleighScattering` _skyatmosphere (`KismetMathLibrary.Conv_ColorToLinearColor` (`self.Atmosphere_Color`))))
    (:`then_5`
      (if (`self.Volumetric_Clouds?`)
        (`|ExecutionSequence`
          (:`then_0`
            (`SceneComponent.SetVisibility` _volumetriccloud true false)
            (`VolumetricCloudComponent.SetLayerBottomAltitude` (`self.VolumetricCloud`) (`self.Volumetric_Cloud_Bottom_Altitude`) :!label _label)
            (`VolumetricCloudComponent.SetLayerHeight` (`self.VolumetricCloud`) (`self.Volumetric_Cloud_Height`))
            (`KismetMaterialLibrary.SetVectorParameterValue` "/Game/Planet_Project/Assets/Materials/MPC_Volumetric_Cloud.MPC_Volumetric_Cloud" "Volumetric_Cloud_Albedo" (`KismetMathLibrary.Conv_ColorToLinearColor` (`self.Volumetric_Cloud_Color`)))
            (`KismetMaterialLibrary.SetVectorParameterValue` "/Game/Planet_Project/Assets/Materials/MPC_Volumetric_Cloud.MPC_Volumetric_Cloud" "Volumetric_Cloud_Extinction" (`KismetMathLibrary.Conv_ColorToLinearColor` (`self.Volumetric_Cloud_Extinction`)))
            (`KismetMaterialLibrary.SetVectorParameterValue` "/Game/Planet_Project/Assets/Materials/MPC_Volumetric_Cloud.MPC_Volumetric_Cloud" "Volumetric_Cloud_Wind_Direction" (`KismetMathLibrary.Conv_VectorToLinearColor` (`self.Volumetric_Cloud_Wind_Direction`))))
          (:`then_1`
            (if (`self.Volumetric_Clouds_High_Quality?`)
              (`KismetSystemLibrary.ExecuteConsoleCommand` "r.VolumetricCloud.HighQualityAerialPerspective 0" null)
              (`KismetSystemLibrary.ExecuteConsoleCommand` "r.VolumetricRenderTarget 0" null)
              (`KismetSystemLibrary.ExecuteConsoleCommand` " r.SkyAtmosphere.FastSkyLUT 0" null)
              (`KismetSystemLibrary.ExecuteConsoleCommand` "r.SkyAtmosphere.AerialPerspectiveLUT.FastApplyOnOpaque 0" null)
              (else
                (`KismetSystemLibrary.ExecuteConsoleCommand` "r.VolumetricCloud.HighQualityAerialPerspective 0" null)
                (`KismetSystemLibrary.ExecuteConsoleCommand` "r.VolumetricRenderTarget 1" null)
                (`KismetSystemLibrary.ExecuteConsoleCommand` " r.SkyAtmosphere.FastSkyLUT 1" null)
                (`KismetSystemLibrary.ExecuteConsoleCommand` "r.SkyAtmosphere.AerialPerspectiveLUT.FastApplyOnOpaque 1" null)))))
        (else
          (`SceneComponent.SetVisibility` _volumetriccloud false false)
          (goto _label))))
    (:`then_6`
      (if (`self.Destroy_Space_Dome?`)
        (`ActorComponent.K2_DestroyComponent` (`self.SM_Skybox_Dome`))
        (else
          (bind _returnvalue_6 (`PrimitiveComponent.CreateDynamicMaterialInstance` (`self.SM_Skybox_Dome`) 0 "/Game/Planet_Project/Assets/Materials/MI_Star_Nebula.MI_Star_Nebula" "None"))
          ;[1 1 1] Set_Textures
          (`MaterialInstanceDynamic.SetTextureParameterValue` _returnvalue_6 "Flow_map" (`self.T_Flow_Map`))
          (`MaterialInstanceDynamic.SetTextureParameterValue` _returnvalue_6 "T_Color" (`self.T_Cubemap_Color`))
          (`MaterialInstanceDynamic.SetTextureParameterValue` _returnvalue_6 "T_Alpha" (`self.T_Cubemap_Alpha`))
          (`MaterialInstanceDynamic.SetTextureParameterValue` _returnvalue_6 "T_Color_Extra_Cubemap" (`self.T_ExtraCubemap_Color`))
          (`MaterialInstanceDynamic.SetTextureParameterValue` _returnvalue_6 "T_Alpha_Extra_Cubemap" (`self.T_ExtraCubemap_Alpha`))
          (`MaterialInstanceDynamic.SetTextureParameterValue` _returnvalue_6 "T_Stars_Near" (`self.T_Near_Stars`))
          (`MaterialInstanceDynamic.SetTextureParameterValue` _returnvalue_6 "T_Stars_Far" (`self.T_Far_Stars`))
          ;[1 1 1] Star_Control
          (`MeshComponent.SetScalarParameterValueOnMaterials` _sm_skybox_dome "Near_Stars_Desaturation" (`self.Near Star Desaturation`))
          (`MeshComponent.SetScalarParameterValueOnMaterials` _sm_skybox_dome "Far_Stars_Desaturation" (`self.Far Star Desaturation`))
          (`MeshComponent.SetScalarParameterValueOnMaterials` _sm_skybox_dome "Near_Stars_intensity" (`self.Near_Stars_intensity`))
          (`MeshComponent.SetScalarParameterValueOnMaterials` _sm_skybox_dome "Far_Stars_intensity" (`self.Far_Stars_intensity`))
          ;[1 1 1] Color_Control
          (`MeshComponent.SetScalarParameterValueOnMaterials` _sm_skybox_dome "Red_Level" (`self.Red Tint`))
          (`MeshComponent.SetScalarParameterValueOnMaterials` _sm_skybox_dome "Green_Level" (`self.Green Tint`))
          (`MeshComponent.SetScalarParameterValueOnMaterials` _sm_skybox_dome "Blue_Level" (`self.Blue Tint`))
          ;[1 1 1] Color_Control_Extra_Cubemap
          (`MeshComponent.SetScalarParameterValueOnMaterials` _sm_skybox_dome "Red_Level_Extra_Cubemap" (`self.Red_Level_Extra_Cubemap`))
          (`MeshComponent.SetScalarParameterValueOnMaterials` _sm_skybox_dome "Green_Level_Extra_Cubemap" (`self.Green_Level_Extra_Cubemap`))
          (`MeshComponent.SetScalarParameterValueOnMaterials` _sm_skybox_dome "Blue_Level_Extra_Cubemap" (`self.Blue_Level_Extra_Cubemap`))
          ;[1 1 1] Visibility_Control
          (`MeshComponent.SetScalarParameterValueOnMaterials` _sm_skybox_dome "Power" (`self.Brightness`))
          (`MeshComponent.SetScalarParameterValueOnMaterials` _sm_skybox_dome "Saturation" (`self.Saturation`))
          (`MeshComponent.SetVectorParameterValueOnMaterials` _sm_skybox_dome "Flow_Direction" (`self.Flow_Direction`))
          (`MeshComponent.SetScalarParameterValueOnMaterials` _sm_skybox_dome "Sun_Mask_Intensity" (`self.Sun_Mask_Threshold`))
          ;[1 1 1] Visibility_Extra_Cubemap
          (`MeshComponent.SetScalarParameterValueOnMaterials` _sm_skybox_dome "Saturation_Extra_Cubemap" (`self.Saturation_Extra_Cubemap`))
          (`MeshComponent.SetScalarParameterValueOnMaterials` _sm_skybox_dome "Power_Extra_Cubemap" (`self.Brightness_Extra_Cubemap`))
          (`MeshComponent.SetScalarParameterValueOnMaterials` _sm_skybox_dome "Cubemap_Rotation" (`self.Cubemap_Rotation`))
          ;[1 1 1] Alpha
          (`MeshComponent.SetScalarParameterValueOnMaterials` _sm_skybox_dome "Alpha_Strenght" (`self.Alpha_Strenght`))
          (`MeshComponent.SetScalarParameterValueOnMaterials` _sm_skybox_dome "Extra_Alpha_Strenght" (`self.Extra_Alpha_Strenght`)))))))